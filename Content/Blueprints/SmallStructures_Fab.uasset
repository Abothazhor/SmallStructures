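; Small Structures fabricator that takes its health and inventory size from game INI options and supports wireless blueprint sharing.
; On BeginPlay the server reads those options after a short delay (initialising BeerBarrelMax but reading FabricatorMax), then refreshes connected sources.
; FabricatorMax's OnRep resizes the inventory.
; GameCompBlueprintSharing handles multi-use entries, net exec commands and source-list updates, with connection changes multicast.
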(event EventBeginPlay
  (bind _gamecomp_blueprintsharing (Variables|Default|GetGameComp_BlueprintSharing))
  (|CallParentFunction)
  (Utilities|FlowControl|Sequence
    (:then_0
      (Utilities|FlowControl|Delay 0 0.5)
      (Networking|SwitchHasAuthority
        (:Authority
          (bind _asshooter_game_mode (Utilities|Casting|CastToShooterGameMode (Game|GetGameMode)))
          (Utilities|FlowControl|Sequence
            (:then_0
              (Class|ShooterGameMode|InitOptionInteger _asshooter_game_mode "" "SmallStructuresHealth" "FabricatorHealth" 2500))
            (:then_1
              (bind _returnvalue (Class|ShooterGameMode|GetIntOptionIni _asshooter_game_mode "SmallStructuresHealth" "FabricatorHealth"))
              (if (Math|Conversions|ToBoolean(Integer) _returnvalue)
                (Variables|Default|SetHealth (Math|Conversions|ToFloat(Integer) _returnvalue))
                (Variables|Default|SetMaxHealth (Math|Conversions|ToFloat(Integer) _returnvalue) false)
                (else
                  (Variables|Default|SetHealth (Variables|Default|GetHealth))
                  (Variables|Default|SetMaxHealth (Variables|Default|GetHealth) false))))))))
    (:then_1
      (Utilities|FlowControl|Delay 0 0.5)
      (Networking|SwitchHasAuthority
        (:Authority
          (bind _asshooter_game_mode_2 (Utilities|Casting|CastToShooterGameMode (Game|GetGameMode)))
          (Utilities|FlowControl|Sequence
            (:then_0
              (Class|ShooterGameMode|InitOptionInteger _asshooter_game_mode_2 "" "SmallStructuresInventory" "BeerBarrelMax" 10))
            (:then_1
              (bind _returnvalue_2 (Class|ShooterGameMode|GetIntOptionIni _asshooter_game_mode_2 "SmallStructuresInventory" "FabricatorMax"))
              (Variables|Default|SetFabricatorMax _returnvalue_2 true))))))
    (:then_2
      (if (not (Variables|Default|GetbIsPreviewStructure))
        (Networking|SwitchHasAuthority
          (:Authority
            (Utilities|FlowControl|Delay 0 1.0)
            (bind _connectedsources (Default|UpdateConnectedSources _gamecomp_blueprintsharing))
            (bind _output_get (Variables|WirelessExchange|SetConnectedWirelessSources _connectedsources true))
            (Default|HandleonRepConnectedSources _gamecomp_blueprintsharing _output_get)))))))

(fn ConstructionScript)

(fn BPNotifyWirelessSourceAdded
  (params (myExchange :type Primal%20Wireless%20Exchange%20Data%20Object%20Reference) (otherContainer :type Primal%20Structure%20Item%20Container%20Object%20Reference))
  (Utilities|IsValid myExchange
    (:Is%20Valid
      (Utilities|IsValid otherContainer
        (:Is%20Valid
          (if (Utilities|Enum|Equal(Enum) (Variables|/Script/ShooterGame.PrimalWirelessExchangeData|GetWirelessType myExchange) "BlueprintSharing")
            (bind _returnvalue (Utilities|Array|AddUnique (Variables|WirelessExchange|GetConnectedWirelessSources) otherContainer))
            (if (>= _returnvalue 0)
              (Class|PrimalActor|MulticastProperty "ConnectedWirelessSources" false)
              (Default|HandleonRepConnectedSources (Variables|Default|GetGameComp_BlueprintSharing) (Variables|WirelessExchange|GetConnectedWirelessSources)))))))))

(fn BPNotifyWirelessSourceRemoved
  (params (myExchange :type Primal%20Wireless%20Exchange%20Data%20Object%20Reference) (otherContainer :type Primal%20Structure%20Item%20Container%20Object%20Reference))
  (Utilities|IsValid otherContainer
    (:Is%20Valid
      (Utilities|IsValid myExchange
        (:Is%20Valid
          (if (Utilities|Enum|Equal(Enum) (Variables|/Script/ShooterGame.PrimalWirelessExchangeData|GetWirelessType myExchange) "BlueprintSharing")
            (bind _returnvalue (Utilities|Array|RemoveItem (Variables|WirelessExchange|GetConnectedWirelessSources) otherContainer))
            (if _returnvalue
              (Class|PrimalActor|MulticastProperty "ConnectedWirelessSources" false)
              (Default|HandleonRepConnectedSources (Variables|Default|GetGameComp_BlueprintSharing) (Variables|WirelessExchange|GetConnectedWirelessSources)))))))))

(fn BPServerHandleNetExecCommand
  (params (FromPC :type Player%20Controller%20Object%20Reference) (CommandName :type Name :default "None") (ExecParams :type BP%20Net%20Exec%20Params%20Structure%20%28by%20ref%29))
  (bind _intparam1 (Utilities|Struct|BreakBPNetExecParams ExecParams))
  (bind _gamecomp_blueprintsharing (Variables|Default|GetGameComp_BlueprintSharing))
  (bind _returnvalue (|CallParentFunction FromPC CommandName ExecParams))
  (Utilities|FlowControl|Sequence
    (:then_0
      (switch name CommandName
        (:UpdateAvailableSources
          (if (Default|CanUpdateAvailableSources _gamecomp_blueprintsharing FromPC)
            (bind _availablesources (Default|UpdateAvailableSources (Variables|Default|GetGameComp_BlueprintSharing)))
            (bind _output_get (Variables|WirelessExchange|SetAvailableWirelessSources _availablesources true))
            (Default|HandleonRepAvailableSources (Variables|Default|GetGameComp_BlueprintSharing) _output_get)))
        (:AddAvailableSource
          (Default|AddSource _gamecomp_blueprintsharing FromPC _intparam1))
        (:RemoveConnectedSource
          (Default|RemoveSource _gamecomp_blueprintsharing FromPC _intparam1))))
    (:then_1
      (return _returnvalue))))

(fn OnRepAvailableWirelessSources
  (Default|HandleonRepAvailableSources (Variables|Default|GetGameComp_BlueprintSharing) (Variables|WirelessExchange|GetAvailableWirelessSources)))

(fn OnRepConnectedWirelessSources
  (Default|HandleonRepConnectedSources (Variables|Default|GetGameComp_BlueprintSharing) (Variables|WirelessExchange|GetConnectedWirelessSources)))

(fn BPGetMultiUseEntries
  (params (ForPC :type Player%20Controller%20Object%20Reference) (MultiUseEntries :type Array%20of%20Multi%20Use%20Entry%20Structures))
  (Default|AddMultiUseEntries (Variables|Default|GetGameComp_BlueprintSharing) ForPC MultiUseEntries)
  (return MultiUseEntries))

(fn BPClientDoMultiUse
  (params (ForPC :type Player%20Controller%20Object%20Reference) (ClientUseIndex :type Integer))
  (Default|ClientDoMultiUse (Variables|Default|GetGameComp_BlueprintSharing) ForPC ClientUseIndex))

(fn OnRepFabricatorMax
  (bind _primalinventorybp_smallstructures_fab (Variables|Default|GetPrimalInventoryBP_SmallStructures_Fab))
  (bind _output_get (Variables|/Script/ShooterGame.PrimalInventoryComponent|SetMaxInventoryItems _primalinventorybp_smallstructures_fab (Variables|Default|GetFabricatorMax)))
  (Variables|/Script/ShooterGame.PrimalInventoryComponent|SetAbsoluteMaxInventoryItems _primalinventorybp_smallstructures_fab _output_get)
  (Class|PrimalInventoryComponent|InventoryRefresh _primalinventorybp_smallstructures_fab)
  (Networking|SwitchHasAuthority
    (:Authority
      (Class|PrimalStructureItemContainer|RefreshInventoryItemCounts))))