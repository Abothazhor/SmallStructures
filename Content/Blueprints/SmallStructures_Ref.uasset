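; Refrigerator structure Blueprint that lets server configuration override its health.
; On BeginPlay, the authority casts the game mode to ShooterGameMode and reads the RefrigeratorHealth integer from the SmallStructuresHealth INI section.
; A non-zero value sets both Health and MaxHealth; otherwise both keep their existing values.
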(event EventBeginPlay
  (|CallParentFunction)
  (Networking|SwitchHasAuthority
    (:Authority
      (bind _asshooter_game_mode (Utilities|Casting|CastToShooterGameMode (Game|GetGameMode)))
      (bind _returnvalue (Class|ShooterGameMode|GetIntOptionIni _asshooter_game_mode "SmallStructuresHealth" "RefrigeratorHealth"))
      (if (Math|Conversions|ToBoolean(Integer) _returnvalue)
        (Variables|Default|SetHealth (Math|Conversions|ToFloat(Integer) _returnvalue))
        (Variables|Default|SetMaxHealth (Math|Conversions|ToFloat(Integer) _returnvalue) false)
        (else
          (Variables|Default|SetHealth (Variables|Default|GetHealth))
          (Variables|Default|SetMaxHealth (Variables|Default|GetHealth) false))))))

(fn ConstructionScript)