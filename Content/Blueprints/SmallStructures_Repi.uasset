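; Tek Replicator structure in an ARK small structures set, a crafting container with powered and unpowered looks.
; On BeginPlay the authority reads an optional health override from the game mode INI.
; Cosmetic color refreshes, when structure colors are unused, build a dynamic material matching activation state, health and saddle placement.
; Finished crafts send a time-throttled exec command to everyone, and clients spawn an effect at the CraftFX socket.
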(event EventBPRefreshedStructureColors
  (|CallParentFunction)
  (Class|KismetSystemLibrary|CanRunCosmeticEvents
    (:Yes
      (if (not (Variables|Default|GetbUsingStructureColors))
        (bind _returnvalue (Rendering|Material|CreateDynamicMaterialInstance (Variables|Default|GetSkeletalMesh1) 0 (select (Variables|Default|GetbContainerActivated) "/Game/PrimalEarth/TekTier/tek_fabricator/Tek_Fabricator_Colorize_MIC.Tek_Fabricator_Colorize_MIC" "/Game/PrimalEarth/TekTier/tek_fabricator/Tek_Fabricator_Colorize_UnPowered_MIC.Tek_Fabricator_Colorize_UnPowered_MIC") "None" :!class /Script/Engine.PrimitiveComponent))
        (Rendering|Material|SetScalarParameterValue _returnvalue "HealthPercent" (Variables|Default|GetLastHealthPercentage) :!class /Script/Engine.MaterialInstanceDynamic)
        (if (and (Utilities|IsValid (Variables|Default|GetSaddleDino)) (Variables|Default|GetbUsesWorldSpaceMaterial))
          (Rendering|Material|SetScalarParameterValue _returnvalue "DisableWorldSpace" 1.0 :!class /Script/Engine.MaterialInstanceDynamic))))))

(event EventBeginPlay
  (|CallParentFunction)
  (Networking|SwitchHasAuthority
    (:Authority
      (bind _asshooter_game_mode (Utilities|Casting|CastToShooterGameMode (Game|GetGameMode)))
      (bind _returnvalue (Class|ShooterGameMode|GetIntOptionIni _asshooter_game_mode "SmallStructuresHealth" "TekReplicatorHealth"))
      (if (Math|Conversions|ToBoolean(Integer) _returnvalue)
        (Variables|Default|SetHealth (Math|Conversions|ToFloat(Integer) _returnvalue))
        (Variables|Default|SetMaxHealth (Math|Conversions|ToFloat(Integer) _returnvalue) false)
        (else
          (Variables|Default|SetHealth (Variables|Default|GetHealth))
          (Variables|Default|SetMaxHealth (Variables|Default|GetHealth) false))))))

(fn ConstructionScript)

(fn NotifyCraftingFinished
  (if (Class|VictoryCore|IsTimeSince 0 (Variables|Default|GetLastCraftingNotificationTime) 1.5 true)
    (Variables|Default|SetLastCraftingNotificationTime (Utilities|Time|GetGameTimeinSeconds))
    (Class|Actor|ServerSendSimpleExecCommandtoEveryone "CraftingFinished" true true false)))

(fn BPClientHandleNetExecCommand
  (params (CommandName :type Name :default "None") (ExecParams :type BP%20Net%20Exec%20Params%20Structure%20%28by%20ref%29) (ForPC :type Player%20Controller%20Object%20Reference))
  (Utilities|FlowControl|Sequence
    (:then_0
      (switch name CommandName
        (:CraftingFinished
          (Game|SpawnActorfromClass "/Game/PrimalEarth/General/TekFabricatorCraftedEmitter.TekFabricatorCraftedEmitter_C" (Transformation|GetSocketTransform (Variables|Default|GetSkeletalMesh1) "CraftFX" "RTS_World") "AlwaysSpawn" "MultiplyWithRoot" 0 "(R=0.000000,G=0.000000,B=0.000000,A=0.000000)" 0))))
    (:then_1
      (return false))))