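; Small Structures Industrial Grinder, a powered inventory structure that breaks items down into a share of their crafting resources.
; Inventory menu entries for item, stack or grind-all send net exec commands to the server, which checks tribe permission before grinding.
; Grinding filters eligible items, substitutes configured resource types and caps returns per grind.
; On BeginPlay the server reads health and slot limit from INI options, with an OnRep updating inventory size.
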(event EventBeginPlay
  (|CallParentFunction)
  (Utilities|FlowControl|Sequence
    (:then_0
      (Networking|SwitchHasAuthority
        (:Authority
          (bind _asshooter_game_mode (Utilities|Casting|CastToShooterGameMode (Game|GetGameMode)))
          (Utilities|FlowControl|Sequence
            (:then_0
              (Class|ShooterGameMode|InitOptionInteger _asshooter_game_mode "" "SmallStructuresHealth" "IndustrialGrinderHealth" 1250))
            (:then_1
              (bind _returnvalue (Class|ShooterGameMode|GetIntOptionIni _asshooter_game_mode "SmallStructuresHealth" "IndustrialGrinderHealth"))
              (if (Math|Conversions|ToBoolean(Integer) _returnvalue)
                (Variables|Default|SetHealth (Math|Conversions|ToFloat(Integer) _returnvalue))
                (Variables|Default|SetMaxHealth (Math|Conversions|ToFloat(Integer) _returnvalue) false)
                (else
                  (Variables|Default|SetHealth (Variables|Default|GetHealth))
                  (Variables|Default|SetMaxHealth (Variables|Default|GetHealth) false))))))))
    (:then_1
      (Networking|SwitchHasAuthority
        (:Authority
          (bind _asshooter_game_mode_2 (Utilities|Casting|CastToShooterGameMode (Game|GetGameMode)))
          (Utilities|FlowControl|Sequence
            (:then_0
              (Class|ShooterGameMode|InitOptionInteger _asshooter_game_mode_2 "" "SmallStructuresInventory" "IndustrialGrinderMax" 60))
            (:then_1
              (bind _returnvalue_2 (Class|ShooterGameMode|GetIntOptionIni _asshooter_game_mode_2 "SmallStructuresInventory" "IndustrialGrinderMax"))
              (Variables|Default|SetIndustrialGrinderMax _returnvalue_2 true))))))))

(fn ConstructionScript)

(fn BPGetMultiUseEntries
  (params (ForPC :type Player%20Controller%20Object%20Reference) (MultiUseEntries :type Array%20of%20Multi%20Use%20Entry%20Structures))
  (Utilities|FlowControl|Sequence
    (:then_0
      (bind _asshooter_player_controller (Utilities|Casting|CastToShooterPlayerController ForPC))
      (bind _returnvalue (Class|ShooterPlayerController|AllowTribeGroupPermission _asshooter_player_controller "STRUCTUREACTIVATE" self))
      (if (Math|Boolean|ANDBoolean _returnvalue (== (Variables|/Script/Engine.Actor|GetTargetingTeam ForPC) (Variables|Default|GetTargetingTeam)) (Variables|Default|GetbContainerActivated))
        (if (Pawn|IsLocalPlayerController _asshooter_player_controller)
          (bind _returnvalue_2 (Class|ShooterPlayerController|GetInventoryUISelectedItemRemote _asshooter_player_controller))
          (bind _returnvalue_3 (Class|VictoryCore|GetDefaultObject _returnvalue_2))
          (bind _asprimal_item (Utilities|Casting|CastToPrimalItem _returnvalue_3)
            (:then
              (bind _isvalid (CallFunction|IsValidGrindingItem _returnvalue_2))
              (if _isvalid
                (Utilities|Array|Add MultiUseEntries (Utilities|Struct|MakeMultiUseEntry (Utilities|String|ToString(Text) (Utilities|Text|FormatText "Grind Selected Item ({TheCount}x)" (Utilities|Text|ToText(Integer) (Variables|/Script/ShooterGame.PrimalItem|GetItemQuantity _asprimal_item)))) 8878 -1000 true true true))
                (if (> (Variables|/Script/ShooterGame.PrimalItem|GetItemQuantity _returnvalue_2) 1)
                  (Utilities|Array|Add MultiUseEntries (Utilities|Struct|MakeMultiUseEntry (Utilities|String|ToString(Text) (Utilities|Text|FormatText "Grind Selected Stack ({Count}x)" (Utilities|Text|ToText(Integer) (Math|Integer|Min(Integer) (Variables|/Script/ShooterGame.PrimalItem|GetItemQuantity _returnvalue_2) (Variables|Default|GetMaxQuantityToGrind))))) 8879 -1000 true true true)))
                (else
                  (bind _isvalid_2 (CallFunction|IsValidforGrindingAll :!label _label))
                  (if _isvalid_2
                    (Utilities|Array|Add MultiUseEntries (Utilities|Struct|MakeMultiUseEntry "Grind All Items" 8878 -1000 true true true))))))
            (:CastFailed
              (goto _label)))
          (else
            (Utilities|Array|Add MultiUseEntries (Utilities|Struct|MakeMultiUseEntry "Secondary Grind" 8878 -1000 true true))
            (Utilities|Array|Add MultiUseEntries (Utilities|Struct|MakeMultiUseEntry "Tertiary Grind" 8879 -1000 true true))))))
    (:then_1
      (return MultiUseEntries))))

(fn BPClientDoMultiUse
  (params (ForPC :type Player%20Controller%20Object%20Reference) (ClientUseIndex :type Integer))
  (bind _asshooter_player_controller (Utilities|Casting|CastToShooterPlayerController ForPC))
  (bind _returnvalue (Class|ShooterPlayerController|GetInventoryUISelectedItemRemote _asshooter_player_controller))
  (switch int ClientUseIndex
    (:8878
      (Utilities|IsValid _returnvalue
        (:Is%20Valid
          (Class|PrimalPlayerController|ClientSendNetExecCommandtoServer _asshooter_player_controller self (Utilities|Name|MakeLiteralName "GrindItem") (Utilities|Struct|MakeBPNetExecParams (.ItemID1 (Class|PrimalItem|BPGetItemID _returnvalue)) (.ItemID2 (Class|PrimalItem|BPGetItemID _returnvalue))) true))
        (:Is%20Not%20Valid
          (Class|PrimalPlayerController|ClientSendNetExecCommandtoServer _asshooter_player_controller self (Utilities|Name|MakeLiteralName "GrindAll") (Utilities|Struct|MakeBPNetExecParams) true))))
    (:8879
      (Utilities|IsValid _returnvalue
        (:Is%20Valid
          (Class|PrimalPlayerController|ClientSendNetExecCommandtoServer _asshooter_player_controller self (Utilities|Name|MakeLiteralName "GrindStack") (Utilities|Struct|MakeBPNetExecParams (.ItemID1 (Class|PrimalItem|BPGetItemID _returnvalue)) (.ItemID2 (Class|PrimalItem|BPGetItemID _returnvalue))) true))))))

(fn BPServerHandleNetExecCommand
  (params (FromPC :type Player%20Controller%20Object%20Reference) (CommandName :type Name :default "None") (ExecParams :type BP%20Net%20Exec%20Params%20Structure%20%28by%20ref%29))
  (bind (_intparam1 _intparam2) (Utilities|Struct|BreakBPNetExecParams ExecParams))
  (Utilities|FlowControl|Sequence
    (:then_0
      (bind _asshooter_player_controller (Utilities|Casting|CastToShooterPlayerController FromPC))
      (bind _returnvalue (Class|ShooterPlayerController|AllowTribeGroupPermission _asshooter_player_controller "STRUCTUREACTIVATE" self))
      (if (and _returnvalue (== (Variables|/Script/Engine.Actor|GetTargetingTeam FromPC) (Variables|Default|GetTargetingTeam)))
        (switch name CommandName
          (:GrindAll
            (CallFunction|GrindAllItems FromPC))
          (:GrindItem
            (bind _returnvalue_2 (Class|PrimalInventoryComponent|BPFindItemwithID (Variables|Default|GetMyInventoryComponent) _intparam1 _intparam2 :!label _label))
            (if (Utilities|IsValid _returnvalue_2)
              (if (Variables|/Script/ShooterGame.PrimalItem|GetbAllowRemovalFromInventory _returnvalue_2)
                (CallFunction|GrindItem _returnvalue_2 _asshooter_player_controller (LocalVariables|GetGrindStack_HNE) false))))
          (:GrindStack
            (LocalVariables|SetGrindStack_HNE true)
            (goto _label)))))
    (:then_1
      (return true))))

(fn GrindItem
  (params (ItemToGrind :type Primal%20Item%20Object%20Reference) (ForPC :type Shooter%20Player%20Controller%20Object%20Reference) (GrindStack :type Boolean) (MuteSound :type Boolean))
  (bind _isvalid (CallFunction|IsValidGrindingItem ItemToGrind))
  (if _isvalid
    (bind _returnvalue (Class|VictoryCore|GetDefaultObject ItemToGrind))
    (bind _asprimal_item (Utilities|Casting|CastToPrimalItem _returnvalue))
    (LocalVariables|SetDefaultQuantity (Variables|/Script/ShooterGame.PrimalItem|GetItemQuantity _asprimal_item))
    (if MuteSound
      _
      (else
        (Class|ShooterPlayerController|ClientPlayLocalSound ForPC "/Game/PrimalEarth/Sound/SFX/Generic/BuzzSaw.BuzzSaw" false)))
    (bind _asprimal_item_2 (Utilities|Casting|CastToPrimalItemClass (Utilities|GetClass ItemToGrind)))
    (LocalVariables|SetQuantityToGrind (Math|Float|Floor (/ (Math|Conversions|ToFloat(Integer) (select GrindStack (Math|Integer|Min(Integer) (Variables|/Script/ShooterGame.PrimalItem|GetItemQuantity ItemToGrind) (Variables|Default|GetMaxQuantityToGrind)) (LocalVariables|GetDefaultQuantity))) (Math|Conversions|ToFloat(Integer) (LocalVariables|GetDefaultQuantity)))))
    (if (> (LocalVariables|GetQuantityToGrind) 0)
      (Class|PrimalInventoryComponent|BPIncrementItemTemplateQuantity (Variables|Default|GetMyInventoryComponent) _asprimal_item_2 (* (LocalVariables|GetQuantityToGrind) (* (LocalVariables|GetDefaultQuantity) -1)) true false true true false false ItemToGrind false)
      (for (_array_element _array_index) (Variables|/Script/ShooterGame.PrimalItem|GetBaseCraftingResourceRequirements ItemToGrind)
        (bind _returnvalue_2 (Class|PrimalItem|GetCraftingResourceRequirement ItemToGrind _array_index))
        (if (> _returnvalue_2 0)
          (bind _returnvalue_3 (Class|VictoryCore|GetClassDefaultObject (Utilities|Struct|BreakCraftingResourceRequirement _array_element)))
          (bind _asprimal_item_3 (Utilities|Casting|CastToPrimalItem _returnvalue_3))
          (if (not (Variables|/Script/ShooterGame.PrimalItem|GetbIsAbstractItem _asprimal_item_3))
            (bind _outitemclass (CallFunction|GetReplacementItem (Utilities|Struct|BreakCraftingResourceRequirement _array_element)))
            (bind _returnvalue_4 (Class|VictoryCore|GetClassDefaultObject _outitemclass))
            (Utilities|IsValid _returnvalue_4
              (:Is%20Valid
                (bind _asprimal_item_4 (Utilities|Casting|CastToPrimalItem _returnvalue_4))
                (if (not (Variables|/Script/ShooterGame.PrimalItem|GetbResourcePreventGivingFromDemolition _asprimal_item_4))
                  (Class|PrimalInventoryComponent|BPIncrementItemTemplateQuantity (Variables|Default|GetMyInventoryComponent) _outitemclass (* (LocalVariables|GetQuantityToGrind) (Math|Integer|Min(Integer) (Math|Float|Ceil (* (Math|Float|Ceil (/ (Math|Conversions|ToFloat(Integer) _returnvalue_2) (Math|Conversions|ToFloat(Integer) (LocalVariables|GetDefaultQuantity)))) (Variables|Default|GetGrindGiveItemsPercent))) (Variables|Default|GetMaxItemsToGivePerGrind))) true false false false false false 0 false))))))))))

(fn IsValidGrindingItem
  (params (ItemToCheck :type Primal%20Item%20Object%20Reference))
  (Utilities|FlowControl|Sequence
    (:then_0
      (Utilities|IsValid ItemToCheck
        (:Is%20Valid
          (bind _returnvalue (Class|VictoryCore|GetDefaultObject ItemToCheck))
          (bind _asprimal_item (Utilities|Casting|CastToPrimalItem _returnvalue))
          (bind _true (CallFunction|HasCraftingRequirementsGreaterThanOne ItemToCheck))
          (LocalVariables|SetretVal (Math|Boolean|ANDBoolean _true (>= (Variables|/Script/ShooterGame.PrimalItem|GetItemQuantity ItemToCheck) (Variables|/Script/ShooterGame.PrimalItem|GetItemQuantity _asprimal_item)) (> (Utilities|Array|Length (Variables|/Script/ShooterGame.PrimalItem|GetBaseCraftingResourceRequirements ItemToCheck)) 0) (not (Variables|/Script/ShooterGame.PrimalItem|GetbIsBlueprint ItemToCheck)) (or (Variables|/Script/ShooterGame.PrimalItem|GetbCanBeBlueprint ItemToCheck) (Variables|/Script/ShooterGame.PrimalItem|GetbForceAllowGrinding ItemToCheck)) (not (Variables|/Script/ShooterGame.PrimalItem|GetbIsCustomRecipe ItemToCheck)) (not (Variables|/Script/ShooterGame.PrimalItem|GetbForcePreventGrinding ItemToCheck)))))))
    (:then_1
      (return (LocalVariables|GetretVal)))))

(fn GetReplacementItem
  (params (InItemClass :type Primal%20Item%20Class%20Reference))
  (bind _grindgiveitemfrom (Variables|Default|GetGrindGiveItemFrom))
  (bind _returnvalue (Utilities|Array|FindItem _grindgiveitemfrom InItemClass))
  (bind _output_get (LocalVariables|SetOutItem InItemClass))
  (Utilities|FlowControl|Sequence
    (:then_0
      (if (>= _returnvalue 0)
        (LocalVariables|SetOutItem (Utilities|Array|Get(acopy) (Variables|Default|GetGrindGiveItemTo) _returnvalue))))
    (:then_1
      (return _output_get))))

(fn HasCraftingRequirementsGreaterThanOne
  (params (InItem :type Primal%20Item%20Object%20Reference))
  (LocalVariables|SetretVal false)
  (bind _array_element (Utilities|Array|ForEachLoopwithBreak (Variables|/Script/ShooterGame.PrimalItem|GetBaseCraftingResourceRequirements InItem) :!label _label)
    (:LoopBody
      (if (> (Utilities|Struct|BreakCraftingResourceRequirement _array_element) 1.0)
        (LocalVariables|SetretVal true)
        (goto _label Break)))
    (:Completed
      (return (LocalVariables|GetretVal)))))

(fn IsValidforGrindingAll
  (Utilities|FlowControl|Sequence
    (:then_0
      (LocalVariables|SetLocalValue false)
      (bind _array_element (Utilities|Array|ForEachLoopwithBreak (Variables|/Script/ShooterGame.PrimalInventoryComponent|GetInventoryItems (Variables|Default|GetMyInventoryComponent)) :!label _label)
        (:LoopBody
          (bind _isvalid (CallFunction|IsValidGrindingItem _array_element))
          (if _isvalid
            (LocalVariables|SetLocalValue true)
            (goto _label Break)))))
    (:then_1
      (return (LocalVariables|GetLocalValue)))))

(fn GrindAllItems
  (params (ForPC :type Player%20Controller%20Object%20Reference))
  (bind _itemstogrind (LocalVariables|GetItemsToGrind))
  (bind _isvalid (CallFunction|IsValidforGrindingAll))
  (if _isvalid
    (bind _asshooter_player_controller (Utilities|Casting|CastToShooterPlayerController ForPC))
    (bind _array_element (Utilities|Array|ForEachLoopwithBreak (Variables|/Script/ShooterGame.PrimalInventoryComponent|GetInventoryItems (Variables|Default|GetMyInventoryComponent)))
      (:LoopBody
        (Utilities|IsValid _array_element
          (:Is%20Valid
            (if (Variables|/Script/ShooterGame.PrimalItem|GetbAllowRemovalFromInventory _array_element)
              (bind _isvalid_2 (CallFunction|IsValidGrindingItem _array_element))
              (if _isvalid_2
                (Utilities|Array|Add (LocalVariables|GetItemsToGrind) _array_element))))))
      (:Completed
        (for _array_element_2 _itemstogrind
          (CallFunction|GrindItem _array_element_2 _asshooter_player_controller true true))
        (if (> (Utilities|Array|Length _itemstogrind) 0)
          (Class|ShooterPlayerController|ClientPlayLocalSound _asshooter_player_controller "/Game/PrimalEarth/Sound/SFX/Generic/BuzzSaw.BuzzSaw" false))))))

(fn OnRepIndustrialGrinderMax
  (bind _primalinventorybp_smallstructures_ig (Variables|Default|GetPrimalInventoryBP_SmallStructures_IG))
  (bind _output_get (Variables|/Script/ShooterGame.PrimalInventoryComponent|SetMaxInventoryItems _primalinventorybp_smallstructures_ig (Variables|Default|GetIndustrialGrinderMax)))
  (Variables|/Script/ShooterGame.PrimalInventoryComponent|SetAbsoluteMaxInventoryItems _primalinventorybp_smallstructures_ig _output_get)
  (Class|PrimalInventoryComponent|InventoryRefresh _primalinventorybp_smallstructures_ig)
  (Networking|SwitchHasAuthority
    (:Authority
      (Class|PrimalStructureItemContainer|RefreshInventoryItemCounts))))