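; Micro refrigerator structure variant whose health and inventory capacity are configurable through the game INI.
; On BeginPlay the server registers default options with ShooterGameMode and reads them back, falling back to current Health if that setting is zero.
; RefrigeratorMax's OnRep pushes capacity into the inventory component's item limits and refreshes it, with the server also refreshing item counts.
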(event EventBeginPlay
  (|CallParentFunction)
  (Utilities|FlowControl|Sequence
    (:then_0
      (Networking|SwitchHasAuthority
        (:Authority
          (bind _asshooter_game_mode (Utilities|Casting|CastToShooterGameMode (Game|GetGameMode)))
          (Utilities|FlowControl|Sequence
            (:then_0
              (Class|ShooterGameMode|InitOptionInteger _asshooter_game_mode "" "SmallStructuresHealth" "MRefrigeratorHealth" 500))
            (:then_1
              (bind _returnvalue (Class|ShooterGameMode|GetIntOptionIni _asshooter_game_mode "SmallStructuresHealth" "MRefrigeratorHealth"))
              (if (Math|Conversions|ToBoolean(Integer) _returnvalue)
                (Variables|Default|SetHealth (Math|Conversions|ToFloat(Integer) _returnvalue))
                (Variables|Default|SetMaxHealth (Math|Conversions|ToFloat(Integer) _returnvalue) false)
                (else
                  (Variables|Default|SetHealth (Variables|Default|GetHealth))
                  (Variables|Default|SetMaxHealth (Variables|Default|GetHealth) false))))))))
    (:then_1
      (Networking|SwitchHasAuthority
        (:Authority
          (bind _asshooter_game_mode_2 (Utilities|Casting|CastToShooterGameMode (Game|GetGameMode)))
          (Utilities|FlowControl|Sequence
            (:then_0
              (Class|ShooterGameMode|InitOptionInteger _asshooter_game_mode_2 "" "SmallStructuresInventory" "MRefrigeratorMax" 40))
            (:then_1
              (bind _returnvalue_2 (Class|ShooterGameMode|GetIntOptionIni _asshooter_game_mode_2 "SmallStructuresInventory" "MRefrigeratorMax"))
              (Variables|Default|SetRefrigeratorMax _returnvalue_2 true))))))))

(fn ConstructionScript)

(fn OnRepRefrigeratorMax
  (bind _primalinventorybp_smallstructures_micro_ref (Variables|Default|GetPrimalInventoryBP_SmallStructures_Micro_Ref))
  (bind _output_get (Variables|/Script/ShooterGame.PrimalInventoryComponent|SetMaxInventoryItems _primalinventorybp_smallstructures_micro_ref (Variables|Default|GetRefrigeratorMax)))
  (Variables|/Script/ShooterGame.PrimalInventoryComponent|SetAbsoluteMaxInventoryItems _primalinventorybp_smallstructures_micro_ref _output_get)
  (Class|PrimalInventoryComponent|InventoryRefresh _primalinventorybp_smallstructures_micro_ref)
  (Networking|SwitchHasAuthority
    (:Authority
      (Class|PrimalStructureItemContainer|RefreshInventoryItemCounts))))