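; Micro water tank structure from a Small Structures set, with server-configurable health, water capacity and inventory slots.
; On BeginPlay the authority registers INI defaults through ShooterGameMode and reads them back, keeping existing health if the setting is zero.
; RepNotify functions apply capacity to MaxWaterAmount and slot count to the inventory component.
; The health option's registered name is garbled and differs from the name read back.
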(event EventBeginPlay
  (|CallParentFunction)
  (Utilities|FlowControl|Sequence
    (:then_0
      (Networking|SwitchHasAuthority
        (:Authority
          (bind _asshooter_game_mode (Utilities|Casting|CastToShooterGameMode (Game|GetGameMode)))
          (Utilities|FlowControl|Sequence
            (:then_0
              (Class|ShooterGameMode|InitOptionFloat _asshooter_game_mode "" "SmallStructuresHealth" "MWaterTMWaterTankHealthankWater" 1.5e+04))
            (:then_1
              (bind _returnvalue (Class|ShooterGameMode|GetIntOptionIni _asshooter_game_mode "SmallStructuresHealth" "MWaterTankHealth"))
              (if (Math|Conversions|ToBoolean(Integer) _returnvalue)
                (Variables|Default|SetHealth (Math|Conversions|ToFloat(Integer) _returnvalue))
                (Variables|Default|SetMaxHealth (Math|Conversions|ToFloat(Integer) _returnvalue) false)
                (else
                  (Variables|Default|SetHealth (Variables|Default|GetHealth))
                  (Variables|Default|SetMaxHealth (Variables|Default|GetHealth) false))))))))
    (:then_1
      (Networking|SwitchHasAuthority
        (:Authority
          (bind _asshooter_game_mode_2 (Utilities|Casting|CastToShooterGameMode (Game|GetGameMode)))
          (Utilities|FlowControl|Sequence
            (:then_0
              (Class|ShooterGameMode|InitOptionFloat _asshooter_game_mode_2 "" "SmallStructuresWater" "MWaterTankWater" 2.5e+03))
            (:then_1
              (bind _returnvalue_2 (Class|ShooterGameMode|GetFloatOptionIni _asshooter_game_mode_2 "SmallStructuresWater" "MWaterTankWater"))
              (Variables|Default|SetWaterTankWater _returnvalue_2 true))))))
    (:then_2
      (Networking|SwitchHasAuthority
        (:Authority
          (bind _asshooter_game_mode_3 (Utilities|Casting|CastToShooterGameMode (Game|GetGameMode)))
          (Utilities|FlowControl|Sequence
            (:then_0
              (Class|ShooterGameMode|InitOptionInteger _asshooter_game_mode_3 "" "SmallStructuresInventory" "MWaterTankMax" 10))
            (:then_1
              (bind _returnvalue_3 (Class|ShooterGameMode|GetIntOptionIni _asshooter_game_mode_3 "SmallStructuresInventory" "MWaterTankMax"))
              (Variables|Default|SetWaterTankMax _returnvalue_3 true))))))))

(fn ConstructionScript
  (|CallParentFunction))

(fn OnRepWaterTankMax
  (bind _primalinventorybp_smallstructures_micro_wt (Variables|Default|GetPrimalInventoryBP_SmallStructures_Micro_WT))
  (bind _output_get (Variables|/Script/ShooterGame.PrimalInventoryComponent|SetMaxInventoryItems _primalinventorybp_smallstructures_micro_wt (Variables|Default|GetWaterTankMax)))
  (Variables|/Script/ShooterGame.PrimalInventoryComponent|SetAbsoluteMaxInventoryItems _primalinventorybp_smallstructures_micro_wt _output_get)
  (Class|PrimalInventoryComponent|InventoryRefresh _primalinventorybp_smallstructures_micro_wt)
  (Networking|SwitchHasAuthority
    (:Authority
      (Class|PrimalStructureItemContainer|RefreshInventoryItemCounts))))

(fn OnRepWaterTankWater
  (Variables|Default|SetMaxWaterAmount (Variables|Default|GetWaterTankWater)))