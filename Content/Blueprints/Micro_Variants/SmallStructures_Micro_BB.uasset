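; Micro beer barrel structure from a Small Structures set, with health, water capacity and inventory size configurable through INI.
; On BeginPlay the authority registers defaults with ShooterGameMode, then reads each setting back.
; RepNotify variables apply water capacity to MaxWaterAmount and the item limit to the inventory component, refreshing it.
; Visual updates toggle the beer particles according to whether the barrel has items.
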(event EventBPUpdateItemVisuals
  (bind _beerparticles (Variables|Default|GetBeerParticles))
  (if (Variables|Default|GetbHasItems)
    (Components|Activation|Activate _beerparticles true)
    (else
      (Components|Activation|Deactivate _beerparticles))))

(event EventBeginPlay
  (|CallParentFunction)
  (Utilities|FlowControl|Sequence
    (:then_0
      (Networking|SwitchHasAuthority
        (:Authority
          (bind _asshooter_game_mode (Utilities|Casting|CastToShooterGameMode (Game|GetGameMode)))
          (Utilities|FlowControl|Sequence
            (:then_0
              (Class|ShooterGameMode|InitOptionInteger _asshooter_game_mode "" "SmallStructuresHealth" "MBeerBarrelHealth" 2500))
            (:then_1
              (bind _returnvalue (Class|ShooterGameMode|GetIntOptionIni _asshooter_game_mode "SmallStructuresHealth" "MBeerBarrelHealth"))
              (if (Math|Conversions|ToBoolean(Integer) _returnvalue)
                (Variables|Default|SetHealth (Math|Conversions|ToFloat(Integer) _returnvalue))
                (Variables|Default|SetMaxHealth (Math|Conversions|ToFloat(Integer) _returnvalue) false)
                (else
                  (Variables|Default|SetHealth (Variables|Default|GetHealth))
                  (Variables|Default|SetMaxHealth (Variables|Default|GetHealth) false))))))))
    (:then_1
      (Networking|SwitchHasAuthority
        (:Authority
          (bind _asshooter_game_mode_2 (Utilities|Casting|CastToShooterGameMode (Game|GetGameMode)))
          (Utilities|FlowControl|Sequence
            (:then_0
              (Class|ShooterGameMode|InitOptionFloat _asshooter_game_mode_2 "" "SmallStructuresWater" "MBeerBarrelWater" 5e+03))
            (:then_1
              (bind _returnvalue_2 (Class|ShooterGameMode|GetFloatOptionIni _asshooter_game_mode_2 "SmallStructuresWater" "MBeerBarrelWater"))
              (Variables|Default|SetBeerBarrelWater _returnvalue_2 false))))))
    (:then_2
      (Networking|SwitchHasAuthority
        (:Authority
          (Class|KismetSystemLibrary|SwitchNetworkMode
            (:Standalone
              _)
            (:DedicatedServer
              _)
            (:ListenServer
              _))
          (bind _asshooter_game_mode_3 (Utilities|Casting|CastToShooterGameMode (Game|GetGameMode)))
          (Utilities|FlowControl|Sequence
            (:then_0
              (Class|ShooterGameMode|InitOptionInteger _asshooter_game_mode_3 "" "SmallStructuresInventory" "MBeerBarrelMax" 10))
            (:then_1
              (bind _returnvalue_3 (Class|ShooterGameMode|GetIntOptionIni _asshooter_game_mode_3 "SmallStructuresInventory" "MBeerBarrelMax"))
              (Variables|Default|SetMicroBeerBarrelMax _returnvalue_3 true))))))))

(fn ConstructionScript)

(fn OnRepBeerBarrelWater
  (Variables|Default|SetMaxWaterAmount (Variables|Default|GetBeerBarrelWater)))

(fn OnRepMicroBeerBarrelMax
  (bind _primalinventorybp_smallstructures_micro_bb (Variables|Default|GetPrimalInventoryBP_SmallStructures_Micro_BB))
  (bind _output_get (Variables|/Script/ShooterGame.PrimalInventoryComponent|SetMaxInventoryItems _primalinventorybp_smallstructures_micro_bb (Variables|Default|GetMicroBeerBarrelMax)))
  (Variables|/Script/ShooterGame.PrimalInventoryComponent|SetAbsoluteMaxInventoryItems _primalinventorybp_smallstructures_micro_bb _output_get)
  (Class|PrimalInventoryComponent|InventoryRefresh _primalinventorybp_smallstructures_micro_bb)
  (Networking|SwitchHasAuthority
    (:Authority
      (Class|PrimalStructureItemContainer|RefreshInventoryItemCounts))))