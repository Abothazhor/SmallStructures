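; Micro vault storage structure from an ARK Small Structures mod, with health and slot count configurable through the server INI.
; On BeginPlay the authority registers default INI options, then applies health (keeping current health if zero) and VaultMax.
; OnRep_VaultMax copies the slot limit into the inventory component's max and absolute max and refreshes it, with the authority also refreshing item counts.
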(event EventBeginPlay
  (|CallParentFunction)
  (Utilities|FlowControl|Sequence
    (:then_0
      (Networking|SwitchHasAuthority
        (:Authority
          (bind _asshooter_game_mode (Utilities|Casting|CastToShooterGameMode (Game|GetGameMode)))
          (Utilities|FlowControl|Sequence
            (:then_0
              (Class|ShooterGameMode|InitOptionInteger _asshooter_game_mode "" "SmallStructuresHealth" "MVaultHealth" 25000))
            (:then_1
              (bind _returnvalue (Class|ShooterGameMode|GetIntOptionIni _asshooter_game_mode "SmallStructuresHealth" "MVaultHealth"))
              (if (Math|Conversions|ToBoolean(Integer) _returnvalue)
                (Variables|Default|SetHealth (Math|Conversions|ToFloat(Integer) _returnvalue))
                (Variables|Default|SetMaxHealth (Math|Conversions|ToFloat(Integer) _returnvalue) false)
                (else
                  (Variables|Default|SetHealth (Variables|Default|GetHealth))
                  (Variables|Default|SetMaxHealth (Variables|Default|GetHealth) false))))))))
    (:then_1
      (Networking|SwitchHasAuthority
        (:Authority
          (bind _asshooter_game_mode_2 (Utilities|Casting|CastToShooterGameMode (Game|GetGameMode)))
          (Utilities|FlowControl|Sequence
            (:then_0
              (Class|ShooterGameMode|InitOptionInteger _asshooter_game_mode_2 "" "SmallStructuresInventory" "MVaultMax" 150))
            (:then_1
              (bind _returnvalue_2 (Class|ShooterGameMode|GetIntOptionIni _asshooter_game_mode_2 "SmallStructuresInventory" "MVaultMax"))
              (Variables|Default|SetVaultMax _returnvalue_2 false))))))))

(fn ConstructionScript)

(fn OnRepVaultMax
  (bind _primalinventorybp_smallstructures_micro_va (Variables|Default|GetPrimalInventoryBP_SmallStructures_Micro_Va))
  (bind _output_get (Variables|/Script/ShooterGame.PrimalInventoryComponent|SetMaxInventoryItems _primalinventorybp_smallstructures_micro_va (Variables|Default|GetVaultMax)))
  (Variables|/Script/ShooterGame.PrimalInventoryComponent|SetAbsoluteMaxInventoryItems _primalinventorybp_smallstructures_micro_va _output_get)
  (Class|PrimalInventoryComponent|InventoryRefresh _primalinventorybp_smallstructures_micro_va)
  (Networking|SwitchHasAuthority
    (:Authority
      (Class|PrimalStructureItemContainer|RefreshInventoryItemCounts))))