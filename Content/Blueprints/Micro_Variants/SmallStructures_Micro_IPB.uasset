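; Micro IndustrialPB crafting structure from the SmallStructures set, with an inventory and a heat visual while active.
; On BeginPlay the server registers and reads game-mode INI options for slot cap, health and crafting speed, ignoring zero for the latter two.
; The replicated slot cap's OnRep resizes and refreshes the inventory.
; Activation toggles heat cosmetically by writing start and target values plus a timestamp into mesh custom primitive data.
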(event EventBeginPlay
  (bind _primalinventorybp_smallstructures_micro_ipb (Variables|Default|GetPrimalInventoryBP_SmallStructures_Micro_IPB))
  (|CallParentFunction)
  (Utilities|FlowControl|Sequence
    (:then_0
      (Networking|SwitchHasAuthority
        (:Authority
          (bind _asshooter_game_mode (Utilities|Casting|CastToShooterGameMode (Game|GetGameMode)))
          (Utilities|FlowControl|Sequence
            (:then_0
              (Class|ShooterGameMode|InitOptionInteger _asshooter_game_mode "" "SmallStructuresInventory" "MIndustrialPBMax" 35))
            (:then_1
              (bind _returnvalue (Class|ShooterGameMode|GetIntOptionIni _asshooter_game_mode "SmallStructuresInventory" "MIndustrialPBMax"))
              (Variables|Default|SetIndustrialPBMax _returnvalue true))))))
    (:then_1
      (Networking|SwitchHasAuthority
        (:Authority
          (bind _asshooter_game_mode_2 (Utilities|Casting|CastToShooterGameMode (Game|GetGameMode)))
          (Utilities|FlowControl|Sequence
            (:then_0
              (Class|ShooterGameMode|InitOptionInteger _asshooter_game_mode_2 "" "SmallStructuresHealth" "MIndustrialPBHealth" 2500))
            (:then_1
              (bind _returnvalue_2 (Class|ShooterGameMode|GetIntOptionIni _asshooter_game_mode_2 "SmallStructuresHealth" "MIndustrialPBHealth"))
              (if (Math|Conversions|ToBoolean(Integer) _returnvalue_2)
                (Variables|Default|SetHealth (Math|Conversions|ToFloat(Integer) _returnvalue_2))
                (Variables|Default|SetMaxHealth (Math|Conversions|ToFloat(Integer) _returnvalue_2) true)
                (else
                  (Variables|Default|SetHealth (Variables|Default|GetHealth))
                  (Variables|Default|SetMaxHealth (Variables|Default|GetHealth) true))))))))
    (:then_2
      (Networking|SwitchHasAuthority
        (:Authority
          (bind _asshooter_game_mode_3 (Utilities|Casting|CastToShooterGameMode (Game|GetGameMode)))
          (Utilities|FlowControl|Sequence
            (:then_0
              (Class|ShooterGameMode|InitOptionInteger _asshooter_game_mode_3 "" "SmallStructuresSpeed" "MIndustrialPBSpeed" 15))
            (:then_1
              (bind _returnvalue_3 (Class|ShooterGameMode|GetIntOptionIni _asshooter_game_mode_3 "SmallStructuresSpeed" "MIndustrialPBSpeed"))
              (if (Math|Conversions|ToBoolean(Integer) _returnvalue_3)
                (Variables|/Script/ShooterGame.PrimalInventoryComponent|SetCraftingItemSpeed _primalinventorybp_smallstructures_micro_ipb (Math|Conversions|ToFloat(Integer) _returnvalue_3))
                (else
                  (Variables|/Script/ShooterGame.PrimalInventoryComponent|SetCraftingItemSpeed _primalinventorybp_smallstructures_micro_ipb (Variables|/Script/ShooterGame.PrimalInventoryComponent|GetCraftingItemSpeed _primalinventorybp_smallstructures_micro_ipb)))))))))
    (:then_3
      (Class|KismetSystemLibrary|CanRunCosmeticEvents
        (:Yes
          (Utilities|FlowControl|Delay 0)
          (if (Variables|Default|GetbContainerActivated)
            (CallFunction|ToggleHeat true)))))))

(fn ConstructionScript)

(fn BPContainerActivated
  (|CallParentFunction)
  (Class|KismetSystemLibrary|CanRunCosmeticEvents
    (:Yes
      (CallFunction|ToggleHeat true))))

(fn BPContainerDeactivated
  (|CallParentFunction)
  (Class|KismetSystemLibrary|CanRunCosmeticEvents
    (:Yes
      (CallFunction|ToggleHeat false))))

(fn ToggleHeat
  (params (TurnOn :type Boolean))
  (bind _mystaticmesh (Variables|Default|GetMyStaticMesh))
  (if TurnOn
    (Rendering|Material|SetScalarParameterforCustomPrimitiveData _mystaticmesh "CurrentHeatPercentage" 0.0)
    (Rendering|Material|SetScalarParameterforCustomPrimitiveData _mystaticmesh "NextHeatPercentage" 1.0)
    (else
      (Rendering|Material|SetScalarParameterforCustomPrimitiveData _mystaticmesh "CurrentHeatPercentage" 1.0)
      (Rendering|Material|SetScalarParameterforCustomPrimitiveData _mystaticmesh "NextHeatPercentage" 0.0)))
  (Rendering|Material|SetCustomPrimitiveDataFloat _mystaticmesh 15 (Utilities|Time|GetRealTimeSeconds)))

(fn OnRepIndustrialPBMax
  (bind _primalinventorybp_smallstructures_micro_ipb (Variables|Default|GetPrimalInventoryBP_SmallStructures_Micro_IPB))
  (bind _output_get (Variables|/Script/ShooterGame.PrimalInventoryComponent|SetMaxInventoryItems _primalinventorybp_smallstructures_micro_ipb (Variables|Default|GetIndustrialPBMax)))
  (Variables|/Script/ShooterGame.PrimalInventoryComponent|SetAbsoluteMaxInventoryItems _primalinventorybp_smallstructures_micro_ipb _output_get)
  (Class|PrimalInventoryComponent|InventoryRefresh _primalinventorybp_smallstructures_micro_ipb)
  (Networking|SwitchHasAuthority
    (:Authority
      (Class|PrimalStructureItemContainer|RefreshInventoryItemCounts))))