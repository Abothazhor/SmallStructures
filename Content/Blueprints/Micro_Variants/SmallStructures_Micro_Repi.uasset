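; Micro Tek Replicator crafting structure from the Small Structures set, sharing blueprints wirelessly with other containers.
; On BeginPlay the server loads health and inventory cap from game-mode INI options, with the cap's OnRep resizing the inventory.
; GameCompBlueprintSharing handles menu entries and source add, remove and refresh, fed by net exec commands and replicated source lists.
; Cosmetics include powered/unpowered materials and a throttled, broadcast crafting-finished effect.
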(event EventBeginPlay
  (bind _gamecomp_blueprintsharing (Variables|Default|GetGameComp_BlueprintSharing))
  (|CallParentFunction)
  (Utilities|FlowControl|Sequence
    (:then_0
      (if (not (Variables|Default|GetbIsPreviewStructure))
        (Networking|SwitchHasAuthority
          (:Authority
            (Utilities|FlowControl|Delay 0 1.0)
            (bind _connectedsources (Default|UpdateConnectedSources _gamecomp_blueprintsharing))
            (bind _output_get (Variables|WirelessExchange|SetConnectedWirelessSources _connectedsources true))
            (Default|HandleonRepConnectedSources _gamecomp_blueprintsharing _output_get)))))
    (:then_1
      (Utilities|FlowControl|Delay 0 0.7)
      (Networking|SwitchHasAuthority
        (:Authority
          (bind _asshooter_game_mode (Utilities|Casting|CastToShooterGameMode (Game|GetGameMode)))
          (Utilities|FlowControl|Sequence
            (:then_0
              (Class|ShooterGameMode|InitOptionInteger _asshooter_game_mode "" "SmallStructuresHealth" "MTekReplicatorHealth" 6250))
            (:then_1
              (bind _returnvalue (Class|ShooterGameMode|GetIntOptionIni _asshooter_game_mode "SmallStructuresHealth" "MTekReplicatorHealth"))
              (if (Math|Conversions|ToBoolean(Integer) _returnvalue)
                (Variables|Default|SetHealth (Math|Conversions|ToFloat(Integer) _returnvalue))
                (Variables|Default|SetMaxHealth (Math|Conversions|ToFloat(Integer) _returnvalue) false)
                (else
                  (Variables|Default|SetHealth (Variables|Default|GetHealth))
                  (Variables|Default|SetMaxHealth (Variables|Default|GetHealth) false))))))))
    (:then_2
      (Utilities|FlowControl|Delay 0 0.7)
      (Networking|SwitchHasAuthority
        (:Authority
          (bind _asshooter_game_mode_2 (Utilities|Casting|CastToShooterGameMode (Game|GetGameMode)))
          (Utilities|FlowControl|Sequence
            (:then_0
              (Class|ShooterGameMode|InitOptionInteger _asshooter_game_mode_2 "" "SmallStructuresInventory" "MTekReplicatorMax" 300))
            (:then_1
              (bind _returnvalue_2 (Class|ShooterGameMode|GetIntOptionIni _asshooter_game_mode_2 "SmallStructuresInventory" "MTekReplicatorMax"))
              (Variables|Default|SetMTekReplicatorMax _returnvalue_2 true))))))))

(event EventBPRefreshedStructureColors
  (|CallParentFunction)
  (Class|KismetSystemLibrary|CanRunCosmeticEvents
    (:Yes
      (if (not (Variables|Default|GetbUsingStructureColors))
        (bind _returnvalue (Rendering|Material|CreateDynamicMaterialInstance (Variables|Default|GetSkeletalMesh1) 0 (select (Variables|Default|GetbContainerActivated) "/Game/PrimalEarth/TekTier/tek_fabricator/Tek_Fabricator_Colorize_MIC.Tek_Fabricator_Colorize_MIC" "/Game/PrimalEarth/TekTier/tek_fabricator/Tek_Fabricator_Colorize_UnPowered_MIC.Tek_Fabricator_Colorize_UnPowered_MIC") "None" :!class /Script/Engine.PrimitiveComponent))
        (Rendering|Material|SetScalarParameterValue _returnvalue "HealthPercent" (Variables|Default|GetLastHealthPercentage) :!class /Script/Engine.MaterialInstanceDynamic)
        (if (and (Utilities|IsValid (Variables|Default|GetSaddleDino)) (Variables|Default|GetbUsesWorldSpaceMaterial))
          (Rendering|Material|SetScalarParameterValue _returnvalue "DisableWorldSpace" 1.0 :!class /Script/Engine.MaterialInstanceDynamic))))))

(fn ConstructionScript)

(fn NotifyCraftingFinished
  (if (Class|VictoryCore|IsTimeSince 0 (Variables|Default|GetLastCraftingNotificationTime) 1.5 true)
    (Variables|Default|SetLastCraftingNotificationTime (Utilities|Time|GetGameTimeinSeconds))
    (Class|Actor|ServerSendSimpleExecCommandtoEveryone "CraftingFinished" true true false)))

(fn BPClientHandleNetExecCommand
  (params (CommandName :type Name :default "None") (ExecParams :type BP%20Net%20Exec%20Params%20Structure%20%28by%20ref%29) (ForPC :type Player%20Controller%20Object%20Reference))
  (Utilities|FlowControl|Sequence
    (:then_0
      (switch name CommandName
        (:CraftingFinished
          (Game|SpawnActorfromClass "/Game/PrimalEarth/General/TekFabricatorCraftedEmitter.TekFabricatorCraftedEmitter_C" (Transformation|GetSocketTransform (Variables|Default|GetSkeletalMesh1) "CraftFX" "RTS_World") "AlwaysSpawn" "MultiplyWithRoot" 0 "(R=0.000000,G=0.000000,B=0.000000,A=0.000000)" 0))))
    (:then_1
      (return false))))

(fn BPNotifyWirelessSourceAdded
  (params (myExchange :type Primal%20Wireless%20Exchange%20Data%20Object%20Reference) (otherContainer :type Primal%20Structure%20Item%20Container%20Object%20Reference))
  (Utilities|IsValid myExchange
    (:Is%20Valid
      (Utilities|IsValid otherContainer
        (:Is%20Valid
          (if (Utilities|Enum|Equal(Enum) (Variables|/Script/ShooterGame.PrimalWirelessExchangeData|GetWirelessType myExchange) "BlueprintSharing")
            (bind _returnvalue (Utilities|Array|AddUnique (Variables|WirelessExchange|GetConnectedWirelessSources) otherContainer))
            (if (>= _returnvalue 0)
              (Class|PrimalActor|MulticastProperty "ConnectedWirelessSources" false)
              (Default|HandleonRepConnectedSources (Variables|Default|GetGameComp_BlueprintSharing) (Variables|WirelessExchange|GetConnectedWirelessSources)))))))))

(fn BPNotifyWirelessSourceRemoved
  (params (myExchange :type Primal%20Wireless%20Exchange%20Data%20Object%20Reference) (otherContainer :type Primal%20Structure%20Item%20Container%20Object%20Reference))
  (Utilities|IsValid otherContainer
    (:Is%20Valid
      (Utilities|IsValid myExchange
        (:Is%20Valid
          (if (Utilities|Enum|Equal(Enum) (Variables|/Script/ShooterGame.PrimalWirelessExchangeData|GetWirelessType myExchange) "BlueprintSharing")
            (bind _returnvalue (Utilities|Array|RemoveItem (Variables|WirelessExchange|GetConnectedWirelessSources) otherContainer))
            (if _returnvalue
              (Class|PrimalActor|MulticastProperty "ConnectedWirelessSources" false)
              (Default|HandleonRepConnectedSources (Variables|Default|GetGameComp_BlueprintSharing) (Variables|WirelessExchange|GetConnectedWirelessSources)))))))))

(fn BPServerHandleNetExecCommand
  (params (FromPC :type Player%20Controller%20Object%20Reference) (CommandName :type Name :default "None") (ExecParams :type BP%20Net%20Exec%20Params%20Structure%20%28by%20ref%29))
  (bind _intparam1 (Utilities|Struct|BreakBPNetExecParams ExecParams))
  (bind _gamecomp_blueprintsharing (Variables|Default|GetGameComp_BlueprintSharing))
  (bind _returnvalue (|CallParentFunction FromPC CommandName ExecParams))
  (Utilities|FlowControl|Sequence
    (:then_0
      (switch name CommandName
        (:UpdateAvailableSources
          (if (Default|CanUpdateAvailableSources _gamecomp_blueprintsharing FromPC)
            (bind _availablesources (Default|UpdateAvailableSources (Variables|Default|GetGameComp_BlueprintSharing)))
            (bind _output_get (Variables|WirelessExchange|SetAvailableWirelessSources _availablesources true))
            (Default|HandleonRepAvailableSources (Variables|Default|GetGameComp_BlueprintSharing) _output_get)))
        (:AddAvailableSource
          (Default|AddSource _gamecomp_blueprintsharing FromPC _intparam1))
        (:RemoveConnectedSource
          (Default|RemoveSource _gamecomp_blueprintsharing FromPC _intparam1))))
    (:then_1
      (return _returnvalue))))

(fn OnRepAvailableWirelessSources
  (Default|HandleonRepAvailableSources (Variables|Default|GetGameComp_BlueprintSharing) (Variables|WirelessExchange|GetAvailableWirelessSources)))

(fn OnRepConnectedWirelessSources
  (Default|HandleonRepConnectedSources (Variables|Default|GetGameComp_BlueprintSharing) (Variables|WirelessExchange|GetConnectedWirelessSources)))

(fn BPClientDoMultiUse
  (params (ForPC :type Player%20Controller%20Object%20Reference) (ClientUseIndex :type Integer))
  (Default|ClientDoMultiUse (Variables|Default|GetGameComp_BlueprintSharing) ForPC ClientUseIndex))

(fn BPGetMultiUseEntries
  (params (ForPC :type Player%20Controller%20Object%20Reference) (MultiUseEntries :type Array%20of%20Multi%20Use%20Entry%20Structures))
  (Default|AddMultiUseEntries (Variables|Default|GetGameComp_BlueprintSharing) ForPC MultiUseEntries)
  (return MultiUseEntries))

(fn OnRepMTekReplicatorMax
  (bind _primalinventorybp_smallstructures_micro_repi (Variables|Default|GetPrimalInventoryBP_SmallStructures_Micro_Repi))
  (bind _output_get (Variables|/Script/ShooterGame.PrimalInventoryComponent|SetMaxInventoryItems _primalinventorybp_smallstructures_micro_repi (Variables|Default|GetMTekReplicatorMax)))
  (Variables|/Script/ShooterGame.PrimalInventoryComponent|SetAbsoluteMaxInventoryItems _primalinventorybp_smallstructures_micro_repi _output_get)
  (Class|PrimalInventoryComponent|InventoryRefresh _primalinventorybp_smallstructures_micro_repi)
  (Networking|SwitchHasAuthority
    (:Authority
      (Class|PrimalStructureItemContainer|RefreshInventoryItemCounts))))