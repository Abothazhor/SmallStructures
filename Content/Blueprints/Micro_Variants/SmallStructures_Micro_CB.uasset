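; Micro chemistry bench structure, a small-structures variant whose inventory size and health are configurable through game INI options.
; On BeginPlay the server registers defaults with ShooterGameMode, reads both values back, and sets Health and MaxHealth directly.
; The inventory limit goes through a RepNotify that resizes and refreshes the inventory component.
; Separate OnRep handlers for structure limit and health exist, but BeginPlay never sets their variables.
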(event EventBeginPlay
  (|CallParentFunction)
  (Utilities|FlowControl|Sequence
    (:then_0
      (Networking|SwitchHasAuthority
        (:Authority
          (bind _asshooter_game_mode (Utilities|Casting|CastToShooterGameMode (Game|GetGameMode)))
          (Utilities|FlowControl|Sequence
            (:then_0
              (Class|ShooterGameMode|InitOptionInteger _asshooter_game_mode "" "SmallStructuresInventory" "MChemistryBenchMax" 50))
            (:then_1
              (bind _returnvalue (Class|ShooterGameMode|GetIntOptionIni _asshooter_game_mode "SmallStructuresInventory" "MChemistryBenchMax"))
              (Variables|Default|SetMChmistryBenchMax _returnvalue true))))))
    (:then_1
      (Networking|SwitchHasAuthority
        (:Authority
          (bind _asshooter_game_mode_2 (Utilities|Casting|CastToShooterGameMode (Game|GetGameMode)))
          (Utilities|FlowControl|Sequence
            (:then_0
              (Class|ShooterGameMode|InitOptionInteger _asshooter_game_mode_2 "" "SmallStructuresHealth" "MChemistryBenchHealth" 1250))
            (:then_1
              (bind _returnvalue_2 (Class|ShooterGameMode|GetIntOptionIni _asshooter_game_mode_2 "SmallStructuresHealth" "MChemistryBenchHealth"))
              (if (Math|Conversions|ToBoolean(Integer) _returnvalue_2)
                (Variables|Default|SetHealth (Math|Conversions|ToFloat(Integer) _returnvalue_2))
                (Variables|Default|SetMaxHealth (Math|Conversions|ToFloat(Integer) _returnvalue_2) false)
                (else
                  (Variables|Default|SetHealth (Variables|Default|GetHealth))
                  (Variables|Default|SetMaxHealth (Variables|Default|GetHealth) false))))))))))

(fn ConstructionScript)

(fn OnRepMChmistryBenchMax
  (bind _primalinventorybp_smallstructures_micro_cb (Variables|Default|GetPrimalInventoryBP_SmallStructures_Micro_CB))
  (bind _output_get (Variables|/Script/ShooterGame.PrimalInventoryComponent|SetMaxInventoryItems _primalinventorybp_smallstructures_micro_cb (Variables|Default|GetMChmistryBenchMax)))
  (Variables|/Script/ShooterGame.PrimalInventoryComponent|SetAbsoluteMaxInventoryItems _primalinventorybp_smallstructures_micro_cb _output_get)
  (Class|PrimalInventoryComponent|InventoryRefresh _primalinventorybp_smallstructures_micro_cb)
  (Networking|SwitchHasAuthority
    (:Authority
      (Class|PrimalStructureItemContainer|RefreshInventoryItemCounts))))

(fn OnRepMChemistryBenchCount
  (Variables|Default|SetLimitMaxStructuresInRangeTypeFlag (Variables|Default|GetChemistryBenchLimit)))

(fn OnRepMChemistryBenchHealth
  (bind _mchemistrybenchhealth (Variables|Default|GetMChemistryBenchHealth))
  (if true
    (Variables|Default|SetHealth _mchemistrybenchhealth)
    (Variables|Default|SetMaxHealth _mchemistrybenchhealth false)
    (else
      (Variables|Default|SetHealth (Variables|Default|GetHealth))
      (Variables|Default|SetMaxHealth (Variables|Default|GetHealth) false))))