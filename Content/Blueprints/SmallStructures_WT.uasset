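; Small Structures water tank structure that lets server INI settings override its health and water capacity.
; On BeginPlay, the authority reads integer options from the SmallStructuresHealth and SmallStructuresWater sections through ShooterGameMode.
; A non-zero value sets both Health and MaxHealth, or MaxWaterAmount.
; Otherwise the existing defaults stay, with MaxHealth set to the current Health.
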(event EventBeginPlay
  (|CallParentFunction)
  (Utilities|FlowControl|Sequence
    (:then_0
      (Networking|SwitchHasAuthority
        (:Authority
          (bind _asshooter_game_mode (Utilities|Casting|CastToShooterGameMode (Game|GetGameMode)))
          (bind _returnvalue (Class|ShooterGameMode|GetIntOptionIni _asshooter_game_mode "SmallStructuresHealth" "WaterTankHealth"))
          (if (Math|Conversions|ToBoolean(Integer) _returnvalue)
            (Variables|Default|SetHealth (Math|Conversions|ToFloat(Integer) _returnvalue))
            (Variables|Default|SetMaxHealth (Math|Conversions|ToFloat(Integer) _returnvalue) false)
            (else
              (Variables|Default|SetHealth (Variables|Default|GetHealth))
              (Variables|Default|SetMaxHealth (Variables|Default|GetHealth) false))))))
    (:then_1
      (Networking|SwitchHasAuthority
        (:Authority
          (bind _asshooter_game_mode_2 (Utilities|Casting|CastToShooterGameMode (Game|GetGameMode)))
          (bind _returnvalue_2 (Class|ShooterGameMode|GetIntOptionIni _asshooter_game_mode_2 "SmallStructuresWater" "WaterTankWater"))
          (if (Math|Conversions|ToBoolean(Integer) _returnvalue_2)
            (Variables|Default|SetMaxWaterAmount (Math|Conversions|ToFloat(Integer) _returnvalue_2))
            (else
              (Variables|Default|SetMaxWaterAmount (Variables|Default|GetMaxWaterAmount)))))))))

(fn ConstructionScript
  (|CallParentFunction))