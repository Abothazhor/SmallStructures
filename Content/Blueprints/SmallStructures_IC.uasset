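; Industrial Cooking Pot structure with toggleable auto-crafting, optionally restricted to one selected blueprint or engram.
; On BeginPlay the server applies INI overrides for health and water capacity, and on save loads polls until the inventory is valid to reapply auto-craft state.
; Multi-use entries toggle auto-craft or send the chosen item class to the server by net exec command.
; RepNotify handlers share one function that switches crafting-queue behavior and flags inventory blueprints for auto-crafting.
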(event EventBeginPlay
  (|CallParentFunction)
  (Utilities|FlowControl|Sequence
    (:then_0
      (Networking|SwitchHasAuthority
        (:Authority
          (bind _asshooter_game_mode (Utilities|Casting|CastToShooterGameMode (Game|GetGameMode)))
          (bind _returnvalue (Class|ShooterGameMode|GetIntOptionIni _asshooter_game_mode "SmallStructuresHealth" "IndustrialCookingPotHealth"))
          (if (Math|Conversions|ToBoolean(Integer) _returnvalue)
            (Variables|Default|SetHealth (Math|Conversions|ToFloat(Integer) _returnvalue))
            (Variables|Default|SetMaxHealth (Math|Conversions|ToFloat(Integer) _returnvalue) false)
            (else
              (Variables|Default|SetHealth (Variables|Default|GetHealth))
              (Variables|Default|SetMaxHealth (Variables|Default|GetHealth) false))))))
    (:then_1
      (Networking|SwitchHasAuthority
        (:Authority
          (bind _asshooter_game_mode_2 (Utilities|Casting|CastToShooterGameMode (Game|GetGameMode)))
          (bind _returnvalue_2 (Class|ShooterGameMode|GetIntOptionIni _asshooter_game_mode_2 "SmallStructuresWater" "IndustrialCookingPotWater"))
          (if (Math|Conversions|ToBoolean(Integer) _returnvalue_2)
            (Variables|Default|SetMaxWaterAmount (Math|Conversions|ToFloat(Integer) _returnvalue_2))
            (else
              (Variables|Default|SetMaxWaterAmount (Variables|Default|GetMaxWaterAmount)))))))
    (:then_2
      (Networking|SwitchHasAuthority
        (:Authority
          (if (Variables|Default|GetbLoadedFromSaveGame)
            (Utilities|IsValid (Variables|Default|GetMyInventoryComponent) :!label _label
              (:Is%20Valid
                (CallFunction|HandleonRepAutoCraftingActivated))
              (:Is%20Not%20Valid
                (Utilities|FlowControl|Delay 0)
                (goto _label)))))))))

(fn ConstructionScript)

(fn BPGetMultiUseEntries
  (params (ForPC :type Player%20Controller%20Object%20Reference) (MultiUseEntries :type Array%20of%20Multi%20Use%20Entry%20Structures))
  (bind _returnvalue (Class|PrimalAutocastFunctions|PCtoSPC ForPC))
  (bind _bautocraftactivated (Variables|Default|GetbAutoCraftActivated))
  (Utilities|FlowControl|Sequence
    (:then_0
      (bind _returnvalue_2 (Class|PrimalStructure|AllowStructureAccess ForPC))
      (if _returnvalue_2
        (Utilities|IsValid (Variables|Default|GetMyInventoryComponent)
          (:Is%20Valid
            (bind _returnvalue_3 (Class|ShooterPlayerController|AllowTribeGroupPermission _returnvalue "STRUCTUREACTIVATE" self))
            (if _returnvalue_3
              (Utilities|Array|Add MultiUseEntries (Utilities|Struct|MakeMultiUseEntry 0 (Utilities|String|Append (Utilities|String|SelectString "Disable " "Enable " (Variables|Default|GetbAutoCraftActivated)) "Auto-Craft") 50020 -1000 false (and (not _bautocraftactivated) (> (Utilities|Array|Length (Variables|/Script/ShooterGame.PrimalInventoryComponent|GetItemCraftQueueEntries (Variables|Default|GetMyInventoryComponent))) 0)) false false false true false false false false false false false false 0 false 0 "(B=175,G=175,R=175,A=255)" "(B=255,G=255,R=255,A=255)" 0.0 0.0 0 -1 -1 (select _bautocraftactivated (Variables|Default|GetDisableAutoCraftIcon) (Variables|Default|GetEnableAutoCraftIcon))))
              (if (Utilities|IsValidClass (Variables|Default|GetAutoCraftItemClass))
                (LocalVariables|SetLocalIsClear true)
                (bind _returnvalue_4 (Class|VictoryCore|GetClassDefaultObject (Variables|Default|GetAutoCraftItemClass)))
                (bind _asprimal_item (Utilities|Casting|CastToPrimalItem _returnvalue_4))
                (LocalVariables|SetLocalItem _asprimal_item)
                (bind (_outitemname _outitemicon _returnvalue_5) (Class|PrimalItem|StaticGetItemNameandIcon (Utilities|GetClass (LocalVariables|GetLocalItem)) true _returnvalue :!label _label))
                (if _returnvalue_5
                  (Utilities|Array|Add MultiUseEntries (Utilities|Struct|MakeMultiUseEntry 0 (Class|KismetStringLibrary|ToUpper (Utilities|String|Append (Utilities|String|SelectString "Clear Auto-Craft Item: " "Set Auto-Craft Item: " (LocalVariables|GetLocalIsClear)) _outitemname)) 50021 -1001 true false false false false false false false false false true true false false 0 false 0 "(B=175,G=175,R=175,A=255)" "(B=255,G=255,R=255,A=255)" 0.0 0.0 0 (Math|Integer|SelectInt 1 0 (Utilities|IsValidClass (Variables|Default|GetAutoCraftItemClass))))))
                (else
                  (bind _returnvalue_6 (Class|ShooterPlayerController|GetInventoryUISelectedItemRemote _returnvalue))
                  (Utilities|IsValid _returnvalue_6
                    (:Is%20Valid
                      (if (or (Variables|/Script/ShooterGame.PrimalItem|GetbIsEngram _returnvalue_6) (Variables|/Script/ShooterGame.PrimalItem|GetbIsBlueprint _returnvalue_6))
                        (LocalVariables|SetLocalIsClear false)
                        (LocalVariables|SetLocalItem _returnvalue_6)
                        (goto _label)))))))))))
    (:then_1
      (return MultiUseEntries))))

(fn BPTryMultiUse
  (params (ForPC :type Player%20Controller%20Object%20Reference) (UseIndex :type Integer))
  (bind _myinventorycomponent (Variables|Default|GetMyInventoryComponent))
  (bind _returnvalue (|CallParentFunction ForPC UseIndex))
  (Utilities|FlowControl|Sequence
    (:then_0
      (switch int UseIndex
        (:50020
          (Utilities|IsValid (Variables|Default|GetMyInventoryComponent)
            (:Is%20Valid
              (bind _output_get (Variables|Default|SetbAutoCraftActivated (not (Variables|Default|GetbAutoCraftActivated)) true))
              (if _output_get
                (Class|PrimalInventoryComponent|CheckforAutoCraftBlueprints _myinventorycomponent)
                (else
                  (Class|PrimalInventoryComponent|StopAllCraftingRepairing _myinventorycomponent))))))))
    (:then_1
      (return _returnvalue))))

(fn BPNotifyInventoryItemChange
  (params (bIsItemAdd :type Boolean) (theItem :type Primal%20Item%20Object%20Reference) (bEquipItem :type Boolean))
  (Utilities|IsValid theItem
    (:Is%20Valid
      (if (or (Variables|/Script/ShooterGame.PrimalItem|GetbIsEngram theItem) (Variables|/Script/ShooterGame.PrimalItem|GetbIsBlueprint theItem))
        (if bIsItemAdd
          (Variables|/Script/ShooterGame.PrimalItem|SetbAutoCraftBlueprint theItem (Variables|Default|GetbAutoCraftActivated))
          (else
            (bind _returnvalue (Class|VictoryCore|PureClassDefaultObject (Utilities|GetClass theItem)))
            (bind _asprimal_item (Utilities|Casting|CastToPrimalItem _returnvalue))
            (Variables|/Script/ShooterGame.PrimalItem|SetbAutoCraftBlueprint theItem (Variables|/Script/ShooterGame.PrimalItem|GetbAutoCraftBlueprint _asprimal_item))))))))

(fn OnRepBAutoCraftActivated
  (CallFunction|HandleonRepAutoCraftingActivated))

(fn HandleonRepAutoCraftingActivated
  (bind _bautocraftactivated (Variables|Default|GetbAutoCraftActivated))
  (bind _myinventorycomponent (Variables|Default|GetMyInventoryComponent))
  (bind _autocraftitemclass (Variables|Default|GetAutoCraftItemClass))
  (bind _returnvalue (not _bautocraftactivated))
  (Utilities|IsValid (Variables|Default|GetMyInventoryComponent)
    (:Is%20Valid
      (Variables|/Script/ShooterGame.PrimalInventoryComponent|SetbUseCraftQueue _myinventorycomponent _returnvalue)
      (Variables|/Script/ShooterGame.PrimalInventoryComponent|SetbConsumeCraftingRepairingRequirementsOnStart _myinventorycomponent _returnvalue)
      (Variables|/Script/ShooterGame.PrimalInventoryComponent|SetbCheckForAutoCraftBlueprints _myinventorycomponent _bautocraftactivated)
      (bind _array_element (Utilities|ForEachRefLoop (Variables|/Script/ShooterGame.PrimalInventoryComponent|GetInventoryItems _myinventorycomponent))
        (:LoopBody
          (if (or (Variables|/Script/ShooterGame.PrimalItem|GetbIsBlueprint _array_element) (Variables|/Script/ShooterGame.PrimalItem|GetbIsEngram _array_element))
            (if (Utilities|IsValidClass _autocraftitemclass)
              (Variables|/Script/ShooterGame.PrimalItem|SetbAutoCraftBlueprint _array_element (== (Utilities|GetClass _array_element) _autocraftitemclass))
              (else
                (Variables|/Script/ShooterGame.PrimalItem|SetbAutoCraftBlueprint _array_element _bautocraftactivated)))))))))

(fn OnRepAutoCraftItemClass
  (CallFunction|HandleonRepAutoCraftingActivated))

(fn BPClientDoMultiUse
  (params (ForPC :type Player%20Controller%20Object%20Reference) (ClientUseIndex :type Integer))
  (bind _returnvalue (Class|PrimalAutocastFunctions|PCtoSPC ForPC))
  (if (== ClientUseIndex 50021)
    (if (Utilities|IsValidClass (Variables|Default|GetAutoCraftItemClass))
      (Class|PrimalPlayerController|ClientSendNetExecCommandtoServer _returnvalue self "SetAutoCraftItemClass" (Utilities|Struct|MakeBPNetExecParams) true)
      (else
        (bind _returnvalue_2 (Class|ShooterPlayerController|GetInventoryUISelectedItemRemote _returnvalue))
        (Utilities|IsValid _returnvalue_2
          (:Is%20Valid
            (if (or (Variables|/Script/ShooterGame.PrimalItem|GetbIsEngram _returnvalue_2) (Variables|/Script/ShooterGame.PrimalItem|GetbIsBlueprint _returnvalue_2))
              (bind _returnvalue_3 (Class|VictoryCore|GetClassDefaultObject (Utilities|GetClass _returnvalue_2)))
              (Class|PrimalPlayerController|ClientSendNetExecCommandtoServer _returnvalue self "SetAutoCraftItemClass" (Utilities|Struct|MakeBPNetExecParams 0 0 0 0 0.0 0.0 0.0 0 _returnvalue_3) true))))))))

(fn BPServerHandleNetExecCommand
  (params (FromPC :type Player%20Controller%20Object%20Reference) (CommandName :type Name :default "None") (ExecParams :type BP%20Net%20Exec%20Params%20Structure%20%28by%20ref%29))
  (Utilities|FlowControl|Sequence
    (:then_0
      (if (== CommandName "SetAutoCraftItemClass")
        (bind _asprimal_item (Utilities|Casting|CastToPrimalItem (.ObjParam1 (Utilities|Struct|BreakBPNetExecParams ExecParams)))
          (:then
            (if (Utilities|IsValidClass (Utilities|GetClass _asprimal_item))
              (Variables|Default|SetAutoCraftItemClass (Utilities|GetClass _asprimal_item) true)
              (else
                (Variables|Default|SetAutoCraftItemClass 0 true :!label _label))))
          (:CastFailed
            (goto _label)))))
    (:then_1
      (return false))))